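; BP_Tunnel is an endless tunnel segment with a rotating holed wall, a health pickup and an enemy.
; Functions randomize the wall mesh and roll, place or remove the pickup, and spawn the enemy by chance.
; Overlaps call BP_Player hit, heal and death logic, and projectiles can destroy the enemy.
; The trigger zone has TunnelSpawner spawn another tunnel, destroys this one and adds a point to the player's score.
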(event `self.HealthMesh.OnComponentBeginOverlap`
  (params (OverlappedComponent :type "PrimitiveComponent Object Reference") (OtherActor :type "Actor Object Reference") (OtherComp :type "PrimitiveComponent Object Reference") (OtherBodyIndex :type Integer) (bFromSweep :type Boolean) (SweepResult :type "HitResult Structure (by ref)"))
  ;[1 1 1] Health Mesh Collision
  (bind _asbp_player (cast `/Game/InfiniteMatrix/Blueprints/BP_Player` OtherActor))
  (`/Game/InfiniteMatrix/Blueprints/BP_Player.ProcessHPHit` _asbp_player)
  (`ActorComponent.K2_DestroyComponent` (`self.HealthMesh`)))

(event `self.EnemyMesh.OnComponentBeginOverlap`
  (params (OverlappedComponent :type "PrimitiveComponent Object Reference") (OtherActor :type "Actor Object Reference") (OtherComp :type "PrimitiveComponent Object Reference") (OtherBodyIndex :type Integer) (bFromSweep :type Boolean) (SweepResult :type "HitResult Structure (by ref)"))
  (bind _asbp_player (cast `/Game/InfiniteMatrix/Blueprints/BP_Player` OtherActor)
    (:`then`
      (`/Game/InfiniteMatrix/Blueprints/BP_Player.ProcessEnemyCollision` _asbp_player)
      (`ActorComponent.K2_DestroyComponent` (`self.EnemyMesh`))
      (if (`/Game/InfiniteMatrix/Blueprints/BP_Player.IsDead` _asbp_player)
        (`/Game/InfiniteMatrix/Blueprints/BP_Player.DisplayRestart` _asbp_player)))
    (:`CastFailed`
      (bind _asbp_projectile (cast `/Game/InfiniteMatrix/Blueprints/BP_Projectile` OtherActor))
      (`/Game/InfiniteMatrix/Blueprints/BP_Projectile.ProcessEnemyHit` _asbp_projectile)
      (`ActorComponent.K2_DestroyComponent` (`self.EnemyMesh`)))))

(event `self.ReceiveTick`
  (params (DeltaSeconds :type "Float (single-precision)"))
  (`SceneComponent.K2_AddLocalRotation` (`self.WallMesh`) (`KismetMathLibrary.MakeRotator` (* DeltaSeconds (`self.RotateSpeed`))) false false))

(event `self.TriggerZone.OnComponentBeginOverlap`
  (params (OverlappedComponent :type "PrimitiveComponent Object Reference") (OtherActor :type "Actor Object Reference") (OtherComp :type "PrimitiveComponent Object Reference") (OtherBodyIndex :type Integer) (bFromSweep :type Boolean) (SweepResult :type "HitResult Structure (by ref)"))
  (bind _asbp_player (cast `/Game/InfiniteMatrix/Blueprints/BP_Player` OtherActor))
  (`/Game/InfiniteMatrix/Blueprints/BP_TunnelSpawner.SpawnTunnelAtSpawnPoint` (`self.TunnelSpawner`))
  (`self.K2_DestroyActor`)
  (`/Game/InfiniteMatrix/Blueprints/BP_Player.AddUpdateScore` _asbp_player 1))

(event `self.WallMesh.OnComponentBeginOverlap`
  (params (OverlappedComponent :type "PrimitiveComponent Object Reference") (OtherActor :type "Actor Object Reference") (OtherComp :type "PrimitiveComponent Object Reference") (OtherBodyIndex :type Integer) (bFromSweep :type Boolean) (SweepResult :type "HitResult Structure (by ref)"))
  (bind _asbp_player (cast `/Game/InfiniteMatrix/Blueprints/BP_Player` OtherActor))
  (bind _isdead (`/Game/InfiniteMatrix/Blueprints/BP_Player.ProcessHit` _asbp_player))
  (if _isdead
    (set `/Game/InfiniteMatrix/Blueprints/BP_Player.IsDead` true _asbp_player)
    (`/Game/InfiniteMatrix/Blueprints/BP_Player.DisplayRestart` _asbp_player)))

(event `self.WallMesh.OnComponentHit`
  (params (HitComponent :type "PrimitiveComponent Object Reference") (OtherActor :type "Actor Object Reference") (OtherComp :type "PrimitiveComponent Object Reference") (NormalImpulse :type "Vector Structure") (Hit :type "HitResult Structure (by ref)"))
  ;[1 1 1] Die when hit wall
)

(fn `RandomizeHPLocation`
  (params (SpawnHP :type Boolean))
  (set `self.Spawn HP` SpawnHP)
  (if SpawnHP
    (`SceneComponent.K2_SetRelativeLocation` (`self.HealthMesh`) (`KismetMathLibrary.MakeVector` (`KismetMathLibrary.RandomFloatInRange` 500.0 2500.0) (`KismetMathLibrary.RandomFloatInRange` -300.0 300.0) (`KismetMathLibrary.RandomFloatInRange` -300.0 300.0)) false false)
    (else
      (`ActorComponent.K2_DestroyComponent` (`self.HealthMesh`)))))

(fn `RandomizeWall`
  (`StaticMeshComponent.SetStaticMesh` (`self.WallMesh`) (select `int` (`KismetMathLibrary.RandomIntegerInRange` 0 3) :`0` "/Game/InfiniteMatrix/Meshes/SM_Hole_01.SM_Hole_01" :`1` "/Game/InfiniteMatrix/Meshes/SM_Hole_02.SM_Hole_02" :`2` "/Game/InfiniteMatrix/Meshes/SM_Hole_03.SM_Hole_03" :`3` "/Game/InfiniteMatrix/Meshes/SM_Hole_04.SM_Hole_04" :!type "StaticMesh Object Reference"))
  (`SceneComponent.K2_AddLocalRotation` (`self.WallMesh`) (`KismetMathLibrary.MakeRotator` (`KismetMathLibrary.RandomFloatInRange` 0.0 360.0)) false false))

(fn `SpawnEnemy`
  (if (== (`KismetMathLibrary.RandomIntegerInRange` 0 2) 0)
    (`SceneComponent.K2_SetRelativeLocation` (`self.EnemyMesh`) (`KismetMathLibrary.MakeVector` (`KismetMathLibrary.RandomFloatInRange` 500.0 2500.0) (`KismetMathLibrary.RandomFloatInRange` -300.0 300.0) (`KismetMathLibrary.RandomFloatInRange` -300.0 300.0)) false false)
    (else
      (`ActorComponent.K2_DestroyComponent` (`self.EnemyMesh`)))))

(fn `UserConstructionScript`)